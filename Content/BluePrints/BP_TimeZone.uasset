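; A time zone volume that changes how fast the main character's timer runs while they stand inside it.
; On overlap it writes its TimeDecreaseSpeed setting to the Timer on the character's player state, and on exit it resets that Timer to Normal.
; The construction script swaps the decal material to match the chosen speed, showing stop, slow, fast or faster zones in the level.
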(event Collision|EventActorBeginOverlap
  (params (OtherActor :type Actor%20Object%20Reference))
  (bind _asbp_main_character (Utilities|Casting|CastToBP_MainCharacter OtherActor))
  (bind _asbp_main_player_state (Utilities|Casting|CastToBP_MainPlayerState (Variables|/Script/Engine.Pawn|GetPlayerState _asbp_main_character)))
  (Variables|/Game/BluePrints/GameMode/BP_MainPlayerState.BP_MainPlayerState_C|SetTimer _asbp_main_player_state (Variables|Default|GetTimeDecreaseSpeed)))

(event Collision|EventActorEndOverlap
  (params (OtherActor :type Actor%20Object%20Reference))
  (bind _asbp_main_character (Utilities|Casting|CastToBP_MainCharacter OtherActor))
  (bind _asbp_main_player_state (Utilities|Casting|CastToBP_MainPlayerState (Variables|/Script/Engine.Pawn|GetPlayerState _asbp_main_character)))
  (Variables|/Game/BluePrints/GameMode/BP_MainPlayerState.BP_MainPlayerState_C|SetTimer _asbp_main_player_state "NewEnumerator1"))

(fn ConstructionScript
  (switch Utilities|FlowControl|Switch|SwitchonENUM_Timer (Variables|Default|GetTimeDecreaseSpeed)
    (:NewEnumerator5
      (LocalVariables|SetTargetMat "/Game/BluePrints/Materials/MTI_StopTimerZone.MTI_StopTimerZone"))
    (:NewEnumerator0
      (LocalVariables|SetTargetMat "/Game/BluePrints/Materials/MTI_SlowTimerZone.MTI_SlowTimerZone"))
    (:NewEnumerator3
      (LocalVariables|SetTargetMat "/Game/BluePrints/Materials/MTI_FastTimerZone.MTI_FastTimerZone"))
    (:NewEnumerator4
      (LocalVariables|SetTargetMat "/Game/BluePrints/Materials/MTI_VeryFastTimerZone.MTI_VeryFastTimerZone")))
  (Rendering|Components|Decal|SetDecalMaterial (Variables|Default|GetDecal) (LocalVariables|GetTargetMat)))