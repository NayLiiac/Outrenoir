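; BP_Interactable is a base interactable actor that registers itself with BP_MainCharacter and shows a press-to-interact prompt while overlapped.
; Begin overlap sets the character's CurrentInteractable to this actor and adds a WPB_PressToInteract widget showing the E key and Verb text.
; End overlap clears that reference and removes the widget, checking for a valid player controller first.
; Interact is an empty function taking a Character, apparently left for subclasses to implement.
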(event EventBeginPlay)

(event Collision|EventActorBeginOverlap
  (params (OtherActor :type Actor%20Object%20Reference))
  (bind _asbp_main_character (Utilities|Casting|CastToBP_MainCharacter OtherActor))
  (Variables|/Game/BluePrints/TMP_Blueprints/GameMode/BP_MainCharacter.BP_MainCharacter_C|SetCurrentInteractable _asbp_main_character self)
  (bind _controller (CallFunction|GetPlayerController))
  (Utilities|IsValid _controller
    (:Is%20Valid
      (bind _returnvalue (UserInterface|CreateWidget "/Game/BluePrints/TMP_Blueprints/HUD/WPB_PressToInteract.WPB_PressToInteract_C" _controller))
      (bind _output_get (Variables|Default|SetUIText%20 _returnvalue))
      (Default|UpdateText _output_get "E" (Variables|Default|GetVerb))
      (UserInterface|Viewport|AddtoViewport _returnvalue 0))))

(event EventTick
  (params (DeltaSeconds :type Float%20%28single-precision%29)))

(event Collision|EventActorEndOverlap
  (params (OtherActor :type Actor%20Object%20Reference))
  (bind _asbp_main_character (Utilities|Casting|CastToBP_MainCharacter OtherActor))
  (Variables|/Game/BluePrints/TMP_Blueprints/GameMode/BP_MainCharacter.BP_MainCharacter_C|SetCurrentInteractable _asbp_main_character 0)
  (bind _controller (CallFunction|GetPlayerController _asbp_main_character))
  (Utilities|IsValid _controller
    (:Is%20Valid
      (Widget|RemovefromParent (Variables|Default|GetUIText%20)))))

(fn ConstructionScript)

(fn Interact
  (params (Character :type BP%20Main%20Character%20Object%20Reference)))

(fn GetPlayerController
  (params (Actor :type Actor%20Object%20Reference))
  (bind _ascharacter (Utilities|Casting|CastToCharacter Actor))
  (bind _asplayer_controller (Utilities|Casting|CastToPlayerController (Pawn|GetController _ascharacter)))
  (return _asplayer_controller))