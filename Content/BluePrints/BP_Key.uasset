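; BP_Key is a key pickup that a player collects by interacting with it.
; Its Interact override calls the parent, casts the interacting character's PlayerState to BP_MainPlayerState, increments NumberOfKey and destroys the actor.
; If the cast fails, the key stays in the world and the count is unchanged.
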(event EventBeginPlay
  (|CallParentFunction) ; This node is disabled and will not be called.\nDrag off pins to build functionality.
)

(event Collision|EventActorBeginOverlap
  (params (OtherActor :type Actor%20Object%20Reference))
  (|CallParentFunction OtherActor) ; This node is disabled and will not be called.\nDrag off pins to build functionality.
)

(event EventTick
  (params (DeltaSeconds :type Float%20%28single-precision%29))
  (|CallParentFunction DeltaSeconds) ; This node is disabled and will not be called.\nDrag off pins to build functionality.
)

(fn ConstructionScript
  (|CallParentFunction))

(fn Interact
  (params (Character :type BP%20Main%20Character%20Object%20Reference))
  (|CallParentFunction 0)
  (bind _asbp_main_player_state (Utilities|Casting|CastToBP_MainPlayerState (Variables|/Script/Engine.Pawn|GetPlayerState Character)))
  (Variables|/Game/BluePrints/GameMode/BP_MainPlayerState.BP_MainPlayerState_C|SetNumberOfKey _asbp_main_player_state (+ (Variables|/Game/BluePrints/GameMode/BP_MainPlayerState.BP_MainPlayerState_C|GetNumberOfKey _asbp_main_player_state) 1))
  (Actor|DestroyActor))