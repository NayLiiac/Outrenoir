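; BP_Lever is an interactable lever that toggles between on and off and signals an array of Target objects.
; Interact, if not Locked, flips Activated, plays or reverses a timeline rolling StaticMesh1, and sends TriggerMessage or UntriggerMessage to each target.
; Locked is set inside the target loops and cleared when the timeline finishes, so a lever with no targets never locks during its swing.
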(event Custom|Switch%20On
  (bind _switchlever (Timeline|Timeline Play)
    (:Update
      (Transformation|SetRelativeRotation (Variables|Default|GetStaticMesh1) (Math|Rotator|MakeRotator _switchlever 0.0 0.0) false false))
    (:Finished
      (Variables|Default|SetLocked false))))

(event Custom|Switch%20Off
  (bind _switchlever (Timeline|Timeline Reverse)
    (:Update
      (Transformation|SetRelativeRotation (Variables|Default|GetStaticMesh1) (Math|Rotator|MakeRotator _switchlever 0.0 0.0) false false))
    (:Finished
      (Variables|Default|SetLocked false))))

(event EventBeginPlay)

(event Collision|EventActorBeginOverlap
  (params (OtherActor :type Actor%20Object%20Reference)))

(event EventTick
  (params (DeltaSeconds :type Float%20%28single-precision%29)))

(fn ConstructionScript)

(fn Interact
  (params (Character :type BP%20Main%20Character%20Object%20Reference))
  (bind _target (Variables|Default|GetTarget))
  (|CallParentFunction Character)
  (if (not (Variables|Default|GetLocked))
    (if (Variables|Default|GetActivated)
      (Variables|Default|SetActivated false)
      (CallFunction|SwitchOff)
      (for _array_element _target
        (Class|BPITriggerable|Untrigger(Message) _array_element)
        (Variables|Default|SetLocked true))
      (else
        (Variables|Default|SetActivated true)
        (CallFunction|Switchon)
        (for _array_element_2 _target
          (Class|BPITriggerable|Trigger(Message) _array_element_2)
          (Variables|Default|SetLocked true))))))