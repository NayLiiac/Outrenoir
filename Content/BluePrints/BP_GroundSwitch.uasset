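; BP_GroundSwitch is a pressure switch that reacts when the first player character steps on or off it.
; Overlap begin and end call TriggerMessage or UntriggerMessage on every valid actor in its Target array.
; A MoveAnimation timeline plays and reverses to move the Cube's relative Z, pressing the switch down and raising it back up.
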(event Collision|EventActorBeginOverlap
  (params (OtherActor :type Actor%20Object%20Reference))
  (if (CallFunction|IsPlayer OtherActor)
    (CallFunction|MoveDown)
    (for _array_element (Variables|Default|GetTarget)
      (Utilities|IsValid _array_element
        (:Is%20Valid
          (Class|BPITriggerable|Trigger(Message) _array_element))))))

(event Collision|EventActorEndOverlap
  (params (OtherActor :type Actor%20Object%20Reference))
  (if (CallFunction|IsPlayer OtherActor)
    (CallFunction|MoveUp)
    (for _array_element (Variables|Default|GetTarget)
      (Utilities|IsValid _array_element
        (:Is%20Valid
          (Class|BPITriggerable|Untrigger(Message) _array_element))))))

(event Custom|Move%20Up
  (bind _z_offset (Timeline|MoveAnimation Reverse)
    (:Update
      (Transformation|SetRelativeLocation (Variables|Default|GetCube) (Math|Vector|MakeVector 0.0 0.0 _z_offset) false false))))

(event Custom|Move%20Down
  (bind _z_offset (Timeline|MoveAnimation Play)
    (:Update
      (Transformation|SetRelativeLocation (Variables|Default|GetCube) (Math|Vector|MakeVector 0.0 0.0 _z_offset) false false))))

(fn ConstructionScript)

(fn IsPlayer
  (params (Player :type Actor%20Object%20Reference))
  (return (== Player (Game|GetPlayerCharacter 0))))