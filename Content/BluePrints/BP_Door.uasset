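; BP_Door is a door actor that swings open or closed according to an IsTriggered flag, set and cleared through its Trigger and UnTrigger functions.
; Tick polls the flag every frame and calls OpenDoor or CloseDoor.
; These play or reverse a timeline whose DoorRotation track drives the relative yaw of the Box component.
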(event EventBeginPlay)

(event Collision|EventActorBeginOverlap
  (params (OtherActor :type Actor%20Object%20Reference)))

(event EventTick
  (params (DeltaSeconds :type Float%20%28single-precision%29))
  (if (Variables|Default|GetIsTriggered)
    (CallFunction|OpenDoor)
    (else
      (CallFunction|CloseDoor))))

(event Custom|OpenDoor
  (bind _doorrotation (Timeline|Timeline_0 Play)
    (:Update
      (Transformation|SetRelativeRotation (Variables|Default|GetBox) (Math|Rotator|MakeRotator 0.0 0.0 _doorrotation) false false))))

(event Custom|CloseDoor
  (bind _doorrotation (Timeline|Timeline_0 Reverse)
    (:Update
      (Transformation|SetRelativeRotation (Variables|Default|GetBox) (Math|Rotator|MakeRotator 0.0 0.0 _doorrotation) false false))))

(fn ConstructionScript)

(fn Trigger
  (Variables|Default|SetIsTriggered true))

(fn UnTrigger
  (Variables|Default|SetIsTriggered false))