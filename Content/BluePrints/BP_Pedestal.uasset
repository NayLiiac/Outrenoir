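; BP_Pedestal is an interactable key pedestal that returns the game to the Menu level once all its locks are filled.
; Its Interact override calls the parent, then reads the key count from the interacting character's BP_MainPlayerState.
; Each valid interaction moves one key from the player to the pedestal, provided the player has keys and locks remain.
; The event graph and construction script add no logic of their own.
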(event EventBeginPlay
  (|CallParentFunction) ; This node is disabled and will not be called.\nDrag off pins to build functionality.
)

(event Collision|EventActorBeginOverlap
  (params (OtherActor :type Actor%20Object%20Reference))
  (|CallParentFunction OtherActor) ; This node is disabled and will not be called.\nDrag off pins to build functionality.
)

(event EventTick
  (params (DeltaSeconds :type Float%20%28single-precision%29))
  (|CallParentFunction DeltaSeconds) ; This node is disabled and will not be called.\nDrag off pins to build functionality.
)

(fn ConstructionScript
  (|CallParentFunction))

(fn Interact
  (params (Character :type BP%20Main%20Character%20Object%20Reference))
  (|CallParentFunction Character)
  (bind _asbp_main_player_state (Utilities|Casting|CastToBP_MainPlayerState (Variables|/Script/Engine.Pawn|GetPlayerState Character)))
  (if (and (> (Variables|/Game/BluePrints/GameMode/BP_MainPlayerState.BP_MainPlayerState_C|GetNumberOfKey _asbp_main_player_state) 0) (< (Variables|Default|GetInsertedKeysNumber) (Variables|Default|GetLockNumber)))
    ;[0 1 0.3023] Increases keys by 1, decreases player keys by one
    (Math|Integer|IncrementInt (Variables|Default|GetInsertedKeysNumber)
      (:%20%20
        (Math|Integer|DecrementInt (Variables|/Game/BluePrints/GameMode/BP_MainPlayerState.BP_MainPlayerState_C|GetNumberOfKey _asbp_main_player_state)
          (:%20%20
            (if (== (Variables|Default|GetInsertedKeysNumber) (Variables|Default|GetLockNumber))
              (Game|OpenLevel(byName) "Menu"))))))))