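; BP_MainGameMode is the game mode that counts down a shared RemainingTime on BP_MainGameState at a rate set by the players.
; Every Tick calls DecreaseTime, which loops over player states and maps each BP_MainPlayerState Timer setting, from Stop to Faster, to a dilation multiplier.
; Each player subtracts an equal share of delta time scaled by that multiplier, so the clock's speed blends all players' settings.
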(event EventTick
  (params (DeltaSeconds :type Float%20%28single-precision%29))
  (CallFunction|DecreaseTime DeltaSeconds))

(fn ConstructionScript)

(fn DecreaseTime
  (params (DeltaTime :type Float%20%28double-precision%29))
  (for _index (range 0 (- (Class|GameplayStatics|GetNumPlayerStates) -1))
    (bind _asbp_main_player_state (Utilities|Casting|CastToBP_MainPlayerState (Game|GetPlayerState _index)))
    (switch Utilities|FlowControl|Switch|SwitchonENUM_Timer (Variables|/Game/BluePrints/TMP_Blueprints/GameMode/BP_MainPlayerState.BP_MainPlayerState_C|GetTimer _asbp_main_player_state)
      (:NewEnumerator5
        (LocalVariables|SetTime%20Reduction (Variables|Default|GetStopDilation)))
      (:NewEnumerator0
        (LocalVariables|SetTime%20Reduction (Variables|Default|GetSlowDilation)))
      (:NewEnumerator1
        (LocalVariables|SetTime%20Reduction 1.0))
      (:NewEnumerator3
        (LocalVariables|SetTime%20Reduction (Variables|Default|GetFastDilation)))
      (:NewEnumerator4
        (LocalVariables|SetTime%20Reduction (Variables|Default|GetFasterDilation))))
    (bind _asbp_main_game_state (Utilities|Casting|CastToBP_MainGameState (Game|GetGameState)))
    (Variables|/Game/BluePrints/TMP_Blueprints/GameMode/BP_MainGameState.BP_MainGameState_C|SetRemainingTime _asbp_main_game_state (- (Variables|/Game/BluePrints/TMP_Blueprints/GameMode/BP_MainGameState.BP_MainGameState_C|GetRemainingTime _asbp_main_game_state) (* (/ DeltaTime (Class|GameplayStatics|GetNumPlayerStates)) (LocalVariables|GetTime%20Reduction))))))